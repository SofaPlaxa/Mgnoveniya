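; BP_ClothTaken is a pickup for a hall item (keys, coat or boots) that the player takes before going out.
; BeginPlay sets its mesh from DT_HallItemsToHang by ItemName and hides DoorToOpen.
; TakeCloth hides the mesh, plays the row's sound and sets the matching flag on BP_FirstPersonCharacter, which tracks progress across items.
; Once all three flags are set, it advances the quest, adds Oleg's monologue and unhides DoorToOpen.
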(event `self.ReceiveBeginPlay`
  (bind _cube (`self.Cube`))
  (bind _returnvalue (`|GetDataTableRow` "/Game/Mgnoveniye/BP/Scene01/DT_HallItemsToHang.DT_HallItemsToHang" (`self.ItemName`))
    (:`then`
      (`PrimitiveComponent.SetMaterial` _cube 0 (`StaticMesh.GetMaterial` (`.ItemToHangModel_7_33DBB3904C6607CC61BFE8861B9C1551` (break `/Game/Mgnoveniye/BP/Scene01/BPS_ItemsToHang` _returnvalue)) 0))
      (`StaticMeshComponent.SetStaticMesh` _cube (`.ItemToHangModel_7_33DBB3904C6607CC61BFE8861B9C1551` (break `/Game/Mgnoveniye/BP/Scene01/BPS_ItemsToHang` _returnvalue)))
      (`self.SetActorHiddenInGame` (`self.DoorToOpen`) true))))

(event `TakeCloth`
  (bind _takenitems (`self.TakenItems`))
  (`SceneComponent.SetVisibility` (`self.Cube`) false false)
  (bind _returnvalue (`|GetDataTableRow` "/Game/Mgnoveniye/BP/Scene01/DT_HallItemsToHang.DT_HallItemsToHang" (`self.ItemName`))
    (:`then`
      (`GameplayStatics.PlaySound2D` (`.ItemHangingSound_20_0C6191EF46B59283B2D22D902330B887` (break `/Game/Mgnoveniye/BP/Scene01/BPS_ItemsToHang` _returnvalue)) 1.0 1.0 0.0 null null)
      (`KismetArrayLibrary.Array_AddUnique` _takenitems (break `/Game/Mgnoveniye/BP/Scene01/BPS_ItemsToHang` _returnvalue))
      (for _array_element _takenitems
        (if (== _array_element "keys")
          (bind _asbp_first_person_character (cast `/Game/FirstPerson/Blueprints/BP_FirstPersonCharacter` (`GameplayStatics.GetPlayerCharacter` 0)))
          (set `/Game/FirstPerson/Blueprints/BP_FirstPersonCharacter.KeysOn` true _asbp_first_person_character)
          (if (and (`/Game/FirstPerson/Blueprints/BP_FirstPersonCharacter.CoatOn` _asbp_first_person_character) (`/Game/FirstPerson/Blueprints/BP_FirstPersonCharacter.BootsOn` _asbp_first_person_character))
            (set `self.AllTaken` true)
            (bind _asbp_first_person_character_2 (cast `/Game/FirstPerson/Blueprints/BP_FirstPersonCharacter` (`GameplayStatics.GetPlayerCharacter` 0) :!label _label))
            (set `/Game/FirstPerson/Blueprints/BP_FirstPersonCharacter.CurrentQuestNumber` 1 _asbp_first_person_character_2)
            (set `/Game/FirstPerson/Blueprints/BP_FirstPersonCharacter.SetNewQuest` true _asbp_first_person_character_2)
            (`/Game/FirstPerson/Blueprints/BP_FirstPersonCharacter.AddMonologue` _asbp_first_person_character_2 "Теперь и выходить можно" "Олег")
            (`self.SetActorHiddenInGame` (`self.DoorToOpen`) false)
            (`KismetSystemLibrary.PrintString` "Hello"))
          (elif (== _array_element "coat")
            (bind _asbp_first_person_character_3 (cast `/Game/FirstPerson/Blueprints/BP_FirstPersonCharacter` (`GameplayStatics.GetPlayerCharacter` 0)))
            (set `/Game/FirstPerson/Blueprints/BP_FirstPersonCharacter.CoatOn` true _asbp_first_person_character_3)
            (if (and (`/Game/FirstPerson/Blueprints/BP_FirstPersonCharacter.KeysOn` _asbp_first_person_character_3) (`/Game/FirstPerson/Blueprints/BP_FirstPersonCharacter.BootsOn` _asbp_first_person_character_3))
              (set `self.AllTaken` true)
              (goto _label))
            (elif (== _array_element "boots")
              (bind _asbp_first_person_character_4 (cast `/Game/FirstPerson/Blueprints/BP_FirstPersonCharacter` (`GameplayStatics.GetPlayerCharacter` 0)))
              (set `/Game/FirstPerson/Blueprints/BP_FirstPersonCharacter.BootsOn` true _asbp_first_person_character_4)
              (if (and (`/Game/FirstPerson/Blueprints/BP_FirstPersonCharacter.KeysOn` _asbp_first_person_character_4) (`/Game/FirstPerson/Blueprints/BP_FirstPersonCharacter.CoatOn` _asbp_first_person_character_4))
                (set `self.AllTaken` true)
                (goto _label)))))))))

(fn `UserConstructionScript`)