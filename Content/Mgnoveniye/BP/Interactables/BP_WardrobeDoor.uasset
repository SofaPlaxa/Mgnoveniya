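; BP_WardrobeDoor is an interactable wardrobe door that swings open and shut on alternate OpenDoor calls.
; Each call plays a sound and a FlipFlop plays or reverses a timeline that lerps the inner door's yaw.
; The first time the timeline finishes, it spawns a BP_MonologueTrigger at the player with Oleg's line about the door not closing fully.
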(event `OpenDoor`
  (bind _returnvalue (`GameplayStatics.GetPlayerCharacter` 0))
  (`GameplayStatics.PlaySound2D` "/Game/Mgnoveniye/SFX/Other/RoomDoor_Cue.RoomDoor_Cue" 1.0 1.0 0.0 null null)
  (`/Engine/EditorBlueprintResources/StandardMacros.FlipFlop`
    (:`A`
      (bind (_direction _openfloat) (`Timeline|DoorOpenTimeline` :!via `PlayFromStart` :!label _label)
        (:`Update`
          (`SceneComponent.K2_SetRelativeRotation` (`self.Door_Inside`) (`KismetMathLibrary.MakeRotator` 0.0 0.0 (`KismetMathLibrary.Lerp` 90.0 20.0 _openfloat)) false false))
        (:`Finished`
          (`/Engine/EditorBlueprintResources/StandardMacros.DoOnce` false
            (:`Completed`
              (`|SpawnActorFromClass` "/Game/Mgnoveniye/UI/Monologue/BP_MonologueTrigger.BP_MonologueTrigger_C" (`KismetMathLibrary.MakeTransform` (`SceneComponent.K2_GetComponentLocation` (`Character.CapsuleComponent` _returnvalue))) "Undefined" "MultiplyWithRoot" null "Олег" "Дверь до конца не закрывается, нужно будет поправить" _returnvalue))))))
    (:`B`
      (goto _label :!via `Reverse`))))

(fn `UserConstructionScript`)