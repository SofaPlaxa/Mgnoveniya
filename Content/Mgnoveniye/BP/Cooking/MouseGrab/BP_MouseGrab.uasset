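; BP_MouseGrab is an unfinished mouse-driven grab tool, in which the G key toggles grab mode and the cursor.
; In that mode, left click runs a debug-drawn complex Visibility trace from the cursor, storing any movable component hit and its distance.
; Releasing the button clears that component and releases the PhysicsHandle.
; The physics-simulation check and Tick drag branch are empty, so nothing is grabbed or moved yet.
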(event `Key|G`
  (params (Key :type "Key Structure"))
  (bind _returnvalue (`GameplayStatics.GetPlayerController` 0))
  (:`Pressed`
    (set `self.GrabMode` (not (`self.GrabMode`)))
    (set `PlayerController.bShowMouseCursor` (not (`PlayerController.bShowMouseCursor` _returnvalue)) _returnvalue)))

(event `Key|LeftMouseButton`
  (params (Key :type "Key Structure"))
  (bind _grabmode (`self.GrabMode`))
  (bind (_worldlocation _worlddirection) (`PlayerController.DeprojectMousePositionToWorld` (`PlayerState.GetPlayerController` (`Pawn.PlayerState` (`GameplayStatics.GetPlayerCharacter` 0)))))
  (:`Pressed`
    (if _grabmode
      (bind (_outhit _returnvalue) (`KismetSystemLibrary.LineTraceSingle` :`Start` _worldlocation :`End` (+ _worldlocation (* _worlddirection 1000.0)) :`TraceChannel` "TraceTypeQuery1" :`bTraceComplex` true :`DrawDebugType` "ForDuration"))
      (if _returnvalue
        (if (`|EnumEquality` (`SceneComponent.Mobility` (`.HitComponent` (`GameplayStatics.BreakHitResult` _outhit))) (enumliteral `EComponentMobility` "Movable"))
          (bind (_bblockinghit _binitialoverlap _time _distance _location _impactpoint _normal _impactnormal _physmat _hitactor _hitcomponent) (`GameplayStatics.BreakHitResult` _outhit))
          (set `self.initialDistanceToComponent` _distance)
          (set `self.DraggedComponent` _hitcomponent)
          (if (`SceneComponent.IsSimulatingPhysics` _hitcomponent "None")
            _)))))
  (:`Released`
    (if _grabmode
      (set `self.DraggedComponent` null)
      (`PhysicsHandleComponent.ReleaseComponent` (`self.PhysicsHandle`)))))

(event `self.ReceiveTick`
  (params (DeltaSeconds :type "Float (single-precision)"))
  (if (`self.GrabMode`)
    (`/Engine/EditorBlueprintResources/StandardMacros.IsValid` (`self.DraggedComponent`))))

(fn `UserConstructionScript`)