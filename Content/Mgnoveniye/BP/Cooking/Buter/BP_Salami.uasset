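; BP_Salami is a cooking ingredient that gets cut into slices when a BP_Knife actor overlaps it.
; On overlap it spawns SlicesAmount BP_SalamiSlice actors at its mesh location and gives each a small randomized sideways and upward physics impulse.
; It then plays the NS_CookingSmoke Niagara effect there and destroys itself.
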(event `self.ReceiveActorBeginOverlap`
  (params (OtherActor :type "Actor Object Reference"))
  (bind _returnvalue (`SceneComponent.K2_GetComponentLocation` (`self.StaticMesh`)))
  (`parent.ReceiveActorBeginOverlap` OtherActor)
  (cast `/Game/Mgnoveniye/BP/Cooking/Buter/BP_Knife` OtherActor)
  (for _ (range 1 (+ (`self.SlicesAmount`) 1))
    (bind _returnvalue_2 (`|SpawnActorFromClass` "/Game/Mgnoveniye/BP/Cooking/Buter/BP_SalamiSlice.BP_SalamiSlice_C" (`KismetMathLibrary.MakeTransform` _returnvalue) "Undefined" "MultiplyWithRoot" null null))
    (`PrimitiveComponent.AddImpulse` (`/Game/Mgnoveniye/BP/Cooking/Buter/BP_FoodItem.StaticMesh` _returnvalue_2) (`KismetMathLibrary.MakeVector` (* (`KismetMathLibrary.RandomFloatInRange` -1.0 1.0) (`KismetMathLibrary.RandomFloatInRange` 5.0 10.0)) (* (`KismetMathLibrary.RandomFloatInRange` -1.0 1.0) (`KismetMathLibrary.RandomFloatInRange` 5.0 10.0)) (`KismetMathLibrary.RandomFloatInRange` 20.0 30.0)) "None" false))
  (`NiagaraFunctionLibrary.SpawnSystemAtLocation` "/Game/Mgnoveniye/BP/Cooking/NS_CookingSmoke.NS_CookingSmoke" _returnvalue)
  (`self.K2_DestroyActor`))

(fn `UserConstructionScript`
  (`parent.UserConstructionScript`))