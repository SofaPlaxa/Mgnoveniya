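; BP_BreadSlice is the bread base of a sandwich in the cooking gameplay, assembled by overlapping it with ingredient slices.
; It accepts a cheese slice first, then two salami slices, in that fixed order.
; Each accepted overlap destroys the ingredient actor and reveals the matching pre-placed Cheese, Meat or Meat1 component, using visibility as assembly state.
; The second salami sets Completed, which blocks further additions.
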(event `self.ReceiveActorBeginOverlap`
  (params (OtherActor :type "Actor Object Reference"))
  (`parent.ReceiveActorBeginOverlap` OtherActor)
  (if (not (`SceneComponent.IsVisible` (`self.Cheese`)))
    (cast `/Game/Mgnoveniye/BP/Cooking/Buter/BP_CheeseSlice` OtherActor)
    (`SceneComponent.SetVisibility` (`self.Cheese`) true false)
    (`self.K2_DestroyActor` OtherActor)
    (else
      (cast `/Game/Mgnoveniye/BP/Cooking/Buter/BP_SalamiSlice` OtherActor)
      (if (not (`SceneComponent.IsVisible` (`self.Meat`)))
        (`SceneComponent.SetVisibility` (`self.Meat`) true false)
        (`self.K2_DestroyActor` OtherActor)
        (elif (not (`self.bCompleted`))
          (`SceneComponent.SetVisibility` (`self.Meat1`) true false)
          (`self.K2_DestroyActor` OtherActor)
          (set `self.bCompleted` true))))))

(fn `UserConstructionScript`
  (`parent.UserConstructionScript`))