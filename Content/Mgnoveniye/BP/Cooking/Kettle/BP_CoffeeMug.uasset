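; Coffee mug for the cooking interaction that is filled with coffee and kettle water, then drunk.
; Overlapping a "Coffee"-tagged actor shows the coffee mesh and sets Coffein.
; A "kettle"-tagged overlap then shows CoffeeWater, activates Niagara and sets CoffeeReady.
; Drinkcoffee plays a slurp sound and hides both components when CoffeeReady is set, but leaves both flags set.
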(event `self.ReceiveActorBeginOverlap`
  (params (OtherActor :type "Actor Object Reference"))
  (if (`self.ActorHasTag` OtherActor "Coffee")
    (if (`SceneComponent.IsVisible` (`self.Coffee`))
      (if (`self.ActorHasTag` OtherActor "kettle") :!label _label
        (if (`self.coffein`)
          (if (not (`SceneComponent.IsVisible` (`self.CoffeeWater`)))
            (`SceneComponent.SetVisibility` (`self.CoffeeWater`) true false)
            (`ActorComponent.Activate` (`self.Niagara`) false)
            (set `self.CoffeeReady` true))))
      (else
        (`SceneComponent.SetVisibility` (`self.Coffee`) true false)
        (set `self.coffein` true)))
    (else
      (goto _label))))

(event `Drink coffee`
  (if (`self.CoffeeReady`)
    (`GameplayStatics.PlaySound2D` "/Game/Mgnoveniye/SFX/TestSound/348645_redafs_slurping-sipping-and-gulp-4__mp3cut_net_.348645_redafs_slurping-sipping-and-gulp-4__mp3cut_net_" 1.0 1.0 0.0 null null)
    (`SceneComponent.SetVisibility` (`self.CoffeeWater`) false false)
    (`SceneComponent.SetVisibility` (`self.Coffee`) false false)))

(fn `UserConstructionScript`)