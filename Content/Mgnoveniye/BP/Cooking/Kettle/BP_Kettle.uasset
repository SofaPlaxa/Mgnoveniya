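; Kettle actor for the cooking gameplay that runs a one-way, timed boil when its StartBoil event fires.
; StartBoil sets the StartBoiling flag and plays a switch-on sound, then after a delay plays a switch-off sound, enables physics on WaterKettle and activates the Niagara effect.
; A second delay later destroys the Niagara component, so the effect is not reusable.
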(event `StartBoil`
  (set `self.StartBoiling` true)
  (`GameplayStatics.PlaySound2D` "/Game/Mgnoveniye/SFX/OldSound/Other/Light_On.Light_On" 1.0 1.0 0.0 null null)
  (`KismetSystemLibrary.Delay` 10.0)
  (`GameplayStatics.PlaySound2D` "/Game/Mgnoveniye/SFX/OldSound/Other/Light_Off.Light_Off" 1.0 1.0 0.0 null null)
  (`PrimitiveComponent.SetSimulatePhysics` (`self.water_kettle`) true)
  (`ActorComponent.Activate` (`self.Niagara`) false)
  (`KismetSystemLibrary.Delay` 15.0)
  (`ActorComponent.K2_DestroyComponent` (`self.Niagara`)))

(fn `UserConstructionScript`)