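; Cooking item actor that the player picks up by mouse and combines with other food to build a sandwich.
; Click and release toggle the pickup flag and the mesh's Pawn collision, with release also dropping the physics handle.
; On overlap, actor tags select the recipe: a Knife slices bread, cheese or salami, and slices merge in stages.
; Each match spawns the result at the touched item's location and destroys the consumed actors.
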(event `self.StaticMesh.OnClicked`
  (params (TouchedComponent :type "PrimitiveComponent Object Reference") (ButtonPressed :type "Key Structure"))
  (set `self.isPickedUp` true)
  (`PrimitiveComponent.SetCollisionResponseToChannel` TouchedComponent "ECC_Pawn" "ECR_Ignore"))

(event `self.StaticMesh.OnReleased`
  (params (TouchedComponent :type "PrimitiveComponent Object Reference") (ButtonReleased :type "Key Structure"))
  (set `self.isPickedUp` false)
  (`PhysicsHandleComponent.ReleaseComponent` (`self.PhysicsHandle`))
  (`PrimitiveComponent.SetCollisionResponseToChannel` TouchedComponent "ECC_Pawn" "ECR_Block"))

(event `self.ReceiveActorBeginOverlap`
  (params (OtherActor :type "Actor Object Reference"))
  (bind _touchedactor (`self.TouchedActor`))
  (bind _touchedactor_2 (`self.TouchedActor`))
  (bind _touchedactor_3 (`self.TouchedActor`))
  (bind _touchedactor_4 (`self.TouchedActor`))
  (bind _touchedactor_5 (`self.TouchedActor`))
  (bind _output_get (set `self.TouchedActor` OtherActor))
  (if (`self.ActorHasTag` _output_get "Food")
    (if (and (`self.ActorHasTag` (`self.TouchedActor`) "Bread") (`self.ActorHasTag` "Knife"))
      (`|SpawnActorFromClass` "/Game/Mgnoveniye/BP/Cooking/BP_BreadSlice.BP_BreadSlice_C" (`KismetMathLibrary.Conv_VectorToTransform` (`self.K2_GetActorLocation` (`self.TouchedActor`))) "Undefined" "MultiplyWithRoot" null null)
      (if (not (`self.ActorHasTag` _touchedactor "Knife"))
        (`self.K2_DestroyActor` _touchedactor))
      (elif (and (`self.ActorHasTag` (`self.TouchedActor`) "Cheese") (`self.ActorHasTag` "Knife"))
        (`|SpawnActorFromClass` "/Game/Mgnoveniye/BP/Cooking/BP_CheeseSlice.BP_CheeseSlice_C" (`KismetMathLibrary.Conv_VectorToTransform` (`self.K2_GetActorLocation` _touchedactor_5)) "Undefined" "MultiplyWithRoot" null null)
        (`self.K2_DestroyActor` _touchedactor_5)
        (elif (and (`self.ActorHasTag` (`self.TouchedActor`) "Salami") (`self.ActorHasTag` "Knife"))
          (`|SpawnActorFromClass` "/Game/Mgnoveniye/BP/Cooking/BP_SalamiSlice.BP_SalamiSlice_C" (`KismetMathLibrary.Conv_VectorToTransform` (`self.K2_GetActorLocation` _touchedactor_3)) "Undefined" "MultiplyWithRoot" null null)
          (`self.K2_DestroyActor` _touchedactor_3)
          (elif (and (`self.ActorHasTag` (`self.TouchedActor`) "BreadSlice") (`self.ActorHasTag` "CheeseSlice"))
            (`|SpawnActorFromClass` "/Game/Mgnoveniye/BP/Cooking/BP_CheeseButer.BP_CheeseButer_C" (`KismetMathLibrary.Conv_VectorToTransform` (`self.K2_GetActorLocation` _touchedactor_4)) "Undefined" "MultiplyWithRoot" null null)
            (`self.K2_DestroyActor` _touchedactor_4)
            (`self.K2_DestroyActor`)
            (elif (and (`self.ActorHasTag` (`self.TouchedActor`) "CheeseBurur") (`self.ActorHasTag` "SalamiSlice"))
              (`|SpawnActorFromClass` "/Game/Mgnoveniye/BP/Cooking/BP_Bururbrot.BP_Bururbrot_C" (`KismetMathLibrary.Conv_VectorToTransform` (`self.K2_GetActorLocation` _touchedactor_2)) "Undefined" "MultiplyWithRoot" null null)
              (`self.K2_DestroyActor` _touchedactor_2)
              (`self.K2_DestroyActor`))))))))

(fn `UserConstructionScript`)