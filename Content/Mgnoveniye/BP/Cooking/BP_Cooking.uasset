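; BP_Cooking is a trigger actor that marks a cooking spot for the first-person player.
; On overlap with BP_FirstPersonCharacter it shows the character's start-cook widget, enables cooking, and passes its Arrow component's world location and rotation as the target cooking camera transform.
; When the overlap ends it hides the widget, disables cooking, and zeroes that camera target.
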(event `self.ReceiveActorBeginOverlap`
  (params (OtherActor :type "Actor Object Reference"))
  (bind _arrow (`self.Arrow`))
  (bind _asbp_first_person_character (cast `/Game/FirstPerson/Blueprints/BP_FirstPersonCharacter` OtherActor))
  (`Widget.SetVisibility` (`/Game/FirstPerson/Blueprints/BP_FirstPersonCharacter.StartCookWB` _asbp_first_person_character) "Visible")
  (set `/Game/FirstPerson/Blueprints/BP_FirstPersonCharacter.CanStartCook` true _asbp_first_person_character)
  (set `/Game/FirstPerson/Blueprints/BP_FirstPersonCharacter.TargetCookCamLoc_0` (`SceneComponent.K2_GetComponentLocation` _arrow) _asbp_first_person_character)
  (set `/Game/FirstPerson/Blueprints/BP_FirstPersonCharacter.TargetCookCamRot` (`SceneComponent.K2_GetComponentRotation` _arrow) _asbp_first_person_character))

(event `self.ReceiveActorEndOverlap`
  (params (OtherActor :type "Actor Object Reference"))
  (bind _asbp_first_person_character (cast `/Game/FirstPerson/Blueprints/BP_FirstPersonCharacter` OtherActor))
  (`Widget.SetVisibility` (`/Game/FirstPerson/Blueprints/BP_FirstPersonCharacter.StartCookWB` _asbp_first_person_character) "Hidden")
  (set `/Game/FirstPerson/Blueprints/BP_FirstPersonCharacter.CanStartCook` false _asbp_first_person_character)
  (set `/Game/FirstPerson/Blueprints/BP_FirstPersonCharacter.TargetCookCamLoc_0` (0.0 0.0 0.0) _asbp_first_person_character)
  (set `/Game/FirstPerson/Blueprints/BP_FirstPersonCharacter.TargetCookCamRot` (struct) _asbp_first_person_character))

(fn `UserConstructionScript`)