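; BP_Salami is a cooking actor that breaks into slices when a knife touches it.
; On overlap with a BP_Knife, it spawns SlicesAmount BP_SalamiSlice actors at its own transform and gives each a random upward, scattered physics impulse.
; It then spawns the NS_CookingSmoke Niagara effect at its location and destroys itself.
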(event `self.ReceiveActorBeginOverlap`
  (params (OtherActor :type "Actor Object Reference"))
  (`parent.ReceiveActorBeginOverlap` OtherActor)
  (cast `/Game/Mgnoveniye/BP/Cooking/BP_Knife` OtherActor)
  (for _ (range 1 (+ (`self.SlicesAmount`) 1))
    (bind _returnvalue (`|SpawnActorFromClass` "/Game/Mgnoveniye/BP/Cooking/BP_SalamiSlice.BP_SalamiSlice_C" (`self.GetTransform`) "Undefined" "MultiplyWithRoot" null null))
    (`PrimitiveComponent.AddImpulse` (`/Game/Mgnoveniye/BP/Cooking/BP_FoodItem.StaticMesh` _returnvalue) (`KismetMathLibrary.MakeVector` (* (`KismetMathLibrary.RandomFloatInRange` -1.0 1.0) (`KismetMathLibrary.RandomFloatInRange` 5.0 10.0)) (* (`KismetMathLibrary.RandomFloatInRange` -1.0 1.0) (`KismetMathLibrary.RandomFloatInRange` 5.0 10.0)) (`KismetMathLibrary.RandomFloatInRange` 20.0 30.0)) "None" false))
  (`NiagaraFunctionLibrary.SpawnSystemAtLocation` "/Game/Mgnoveniye/BP/Cooking/NS_CookingSmoke.NS_CookingSmoke" (`self.K2_GetActorLocation`))
  (`self.K2_DestroyActor`))

(fn `UserConstructionScript`
  (`parent.UserConstructionScript`))