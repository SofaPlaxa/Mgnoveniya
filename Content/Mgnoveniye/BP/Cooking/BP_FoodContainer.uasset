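; BP_FoodContainer is an uncooked food container that cooks when placed inside a BP_Microwave.
; Box overlaps with components tagged inMicrowave track whether it is inside, and Tick starts a one-time cook once the door is closed.
; Cooking locks the door and runs a delayed sequence with microwave sounds and a player monologue line about the news.
; It then unlocks the door, spawns BP_FoodContainerCooked at its cube's location and destroys itself.
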(event `self.ReceiveTick`
  (params (DeltaSeconds :type "Float (single-precision)"))
  (if (not (`self.Cooked`))
    (bind _asbp_microwave (cast `/Game/Mgnoveniye/BP/Cooking/Microwave/BP_Microwave` (`self.Microwave`)))
    (if (and (`/Game/Mgnoveniye/BP/Cooking/Microwave/BP_Microwave.doorClosed` _asbp_microwave) (`self.isInside`))
      (set `/Game/Mgnoveniye/BP/Cooking/Microwave/BP_Microwave.canOpenDoor` false _asbp_microwave)
      (set `self.Cooked` true)
      (`self.StartTimer`))))

(event `StartTimer`
  (bind _asbp_microwave (cast `/Game/Mgnoveniye/BP/Cooking/Microwave/BP_Microwave` (`self.Microwave`)))
  (`GameplayStatics.PlaySoundAtLocation` "/Game/Mgnoveniye/SFX/OldSound/Other/Microwave_.Microwave_" (`SceneComponent.K2_GetComponentLocation` (`self.Cube`)) (struct) 1.0 1.0 0.0 null null null null)
  (`KismetSystemLibrary.Delay` 5.0)
  (bind _asbp_first_person_character (cast `/Game/FirstPerson/Blueprints/BP_FirstPersonCharacter` (`GameplayStatics.GetPlayerCharacter` 0)))
  (`/Game/FirstPerson/Blueprints/BP_FirstPersonCharacter.AddMonologue` _asbp_first_person_character "Уже поздновато... сейчас  как раз должны начаться новости" "Олег")
  (`KismetSystemLibrary.Delay` 10.0)
  (`GameplayStatics.PlaySoundAtLocation` "/Game/Mgnoveniye/SFX/OldSound/Other/Microwave_beep.Microwave_beep" (`SceneComponent.K2_GetComponentLocation` (`self.Cube`)) (struct) 1.0 1.0 0.0 null null null null)
  (set `/Game/Mgnoveniye/BP/Cooking/Microwave/BP_Microwave.canOpenDoor` true _asbp_microwave)
  (`|SpawnActorFromClass` "/Game/Mgnoveniye/BP/Cooking/BP_FoodContainerCooked.BP_FoodContainerCooked_C" (`KismetMathLibrary.MakeTransform` (`SceneComponent.K2_GetComponentLocation` (`self.Cube`)) (struct) (`SceneComponent.K2_GetComponentScale` (`self.Cube`))) "Undefined" "MultiplyWithRoot" null null)
  (`self.K2_DestroyActor`))

(event `self.Box.OnComponentBeginOverlap`
  (params (OverlappedComponent :type "PrimitiveComponent Object Reference") (OtherActor :type "Actor Object Reference") (OtherComp :type "PrimitiveComponent Object Reference") (OtherBodyIndex :type Integer) (bFromSweep :type Boolean) (SweepResult :type "HitResult Structure (by ref)"))
  (if (`ActorComponent.ComponentHasTag` OtherComp "inMicrowave")
    (bind _output_get (set `self.Microwave` OtherActor))
    (cast `/Game/Mgnoveniye/BP/Cooking/Microwave/BP_Microwave` _output_get)
    (set `self.isInside` true)
    (`KismetSystemLibrary.PrintString` "is inside")))

(event `self.Box.OnComponentEndOverlap`
  (params (OverlappedComponent :type "PrimitiveComponent Object Reference") (OtherActor :type "Actor Object Reference") (OtherComp :type "PrimitiveComponent Object Reference") (OtherBodyIndex :type Integer))
  (if (`ActorComponent.ComponentHasTag` OtherComp "inMicrowave")
    (bind _output_get (set `self.Microwave` OtherActor))
    (cast `/Game/Mgnoveniye/BP/Cooking/Microwave/BP_Microwave` _output_get)
    (set `self.isInside` false)
    (`KismetSystemLibrary.PrintString` "not inside")))

(fn `UserConstructionScript`)