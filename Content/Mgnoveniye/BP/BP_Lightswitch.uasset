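; BP_Lightswitch is a light switch that turns a referenced LightSource actor on or off.
; Its LightOn and LightOff events show or hide that actor in game, flip the Cube component by offsetting world roll and yaw half a turn with pitch zeroed, and update the LightIsOn flag.
; Neither event checks the current state, and nothing in this graph calls them.
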(event `LightOff`
  (bind _cube (`self.Cube`))
  (bind (_returnvalue_roll _returnvalue_pitch _returnvalue_yaw) (`KismetMathLibrary.BreakRotator` (`SceneComponent.K2_GetComponentRotation` _cube)))
  (`self.SetActorHiddenInGame` (`self.LightSource`) true)
  (`SceneComponent.K2_SetWorldRotation` _cube (`KismetMathLibrary.MakeRotator` (- _returnvalue_roll 180.0) 0.0 (- _returnvalue_yaw 180.0)) false false)
  (set `self.LightIsOn` false))

(event `LightOn`
  (bind _cube (`self.Cube`))
  (bind (_returnvalue_roll _returnvalue_pitch _returnvalue_yaw) (`KismetMathLibrary.BreakRotator` (`SceneComponent.K2_GetComponentRotation` _cube)))
  (`self.SetActorHiddenInGame` (`self.LightSource`) false)
  (`SceneComponent.K2_SetWorldRotation` _cube (`KismetMathLibrary.MakeRotator` (+ _returnvalue_roll 180.0) 0.0 (+ _returnvalue_yaw 180.0)) false false)
  (set `self.LightIsOn` true))

(fn `UserConstructionScript`)