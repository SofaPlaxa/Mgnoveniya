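; BP_RoomItemSlot1 is a Scene01 slot where the player hangs clothing: tie, pants or shirt.
; HangItem looks up HangingItemName in DT_RoomItemsToHang, plays its sound, shows its mesh and records its name.
; Each recorded name clears the matching worn flag on BP_FirstPersonCharacter.
; Once all three are off, it sets AllInPlace and triggers quest 1 on the character; later calls only print a debug message.
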(event `HangItem`
  (bind _hangingitems (`self.HangingItems`))
  (if (`self.AllInPlace`)
    (`KismetSystemLibrary.PrintString` "all in place true")
    (else
      (bind _returnvalue (`|GetDataTableRow` "/Game/Mgnoveniye/BP/Scene01/DT_RoomItemsToHang.DT_RoomItemsToHang" (`self.HangingItemName`))
        (:`then`
          (`GameplayStatics.PlaySound2D` (`.ItemHangingSound_20_0C6191EF46B59283B2D22D902330B887` (break `/Game/Mgnoveniye/BP/Scene01/BPS_ItemsToHang` _returnvalue)) 1.0 1.0 0.0 null null)
          (`StaticMeshComponent.SetStaticMesh` (`self.Cube`) (`.ItemToHangModel_7_33DBB3904C6607CC61BFE8861B9C1551` (break `/Game/Mgnoveniye/BP/Scene01/BPS_ItemsToHang` _returnvalue)))
          (`SceneComponent.SetVisibility` (`self.Cube`) true false)
          (`KismetArrayLibrary.Array_AddUnique` _hangingitems (break `/Game/Mgnoveniye/BP/Scene01/BPS_ItemsToHang` _returnvalue))
          (for _array_element _hangingitems
            (if (== _array_element "tie")
              (bind _asbp_first_person_character (cast `/Game/FirstPerson/Blueprints/BP_FirstPersonCharacter` (`GameplayStatics.GetPlayerCharacter` 0)))
              (set `/Game/FirstPerson/Blueprints/BP_FirstPersonCharacter.TieOn` false _asbp_first_person_character)
              (set `self.ItemHanging` true)
              (if (not (or (`/Game/FirstPerson/Blueprints/BP_FirstPersonCharacter.PantsOn` _asbp_first_person_character) (`/Game/FirstPerson/Blueprints/BP_FirstPersonCharacter.ShirtOn` _asbp_first_person_character)))
                (set `self.AllInPlace` true)
                (bind _asbp_first_person_character_2 (cast `/Game/FirstPerson/Blueprints/BP_FirstPersonCharacter` (`GameplayStatics.GetPlayerCharacter` 0) :!label _label))
                (set `/Game/FirstPerson/Blueprints/BP_FirstPersonCharacter.CurrentQuestNumber` 1 _asbp_first_person_character_2)
                (set `/Game/FirstPerson/Blueprints/BP_FirstPersonCharacter.SetNewQuest` true _asbp_first_person_character_2))
              (elif (== _array_element "pants")
                (bind _asbp_first_person_character_3 (cast `/Game/FirstPerson/Blueprints/BP_FirstPersonCharacter` (`GameplayStatics.GetPlayerCharacter` 0)))
                (set `/Game/FirstPerson/Blueprints/BP_FirstPersonCharacter.PantsOn` false _asbp_first_person_character_3)
                (set `self.ItemHanging` true)
                (if (not (or (`/Game/FirstPerson/Blueprints/BP_FirstPersonCharacter.TieOn` _asbp_first_person_character_3) (`/Game/FirstPerson/Blueprints/BP_FirstPersonCharacter.ShirtOn` _asbp_first_person_character_3)))
                  (set `self.AllInPlace` true)
                  (goto _label))
                (elif (== _array_element "shirt")
                  (bind _asbp_first_person_character_4 (cast `/Game/FirstPerson/Blueprints/BP_FirstPersonCharacter` (`GameplayStatics.GetPlayerCharacter` 0)))
                  (set `/Game/FirstPerson/Blueprints/BP_FirstPersonCharacter.ShirtOn` false _asbp_first_person_character_4)
                  (set `self.ItemHanging` true)
                  (if (not (or (`/Game/FirstPerson/Blueprints/BP_FirstPersonCharacter.TieOn` _asbp_first_person_character_4) (`/Game/FirstPerson/Blueprints/BP_FirstPersonCharacter.PantsOn` _asbp_first_person_character_4)))
                    (set `self.AllInPlace` true)
                    (goto _label)))))))))))

(fn `UserConstructionScript`)