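; BP_OfficeWorker is an office worker that moves in a straight line from its starting position when play begins.
; BeginPlay stores the spawn location and computes a target DistanceToMove along the worker's forward vector.
; The MoveToLocationTL timeline then drives a lerp between the two points, setting the location directly without sweep, collision-aware movement or navigation.
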(event `self.ReceiveBeginPlay`
  (bind _returnvalue (`self.K2_GetActorLocation`))
  (set `self.SpawnWorkerLocation` _returnvalue)
  (set `self.TargetWorkerLoc` (+ _returnvalue (* (`self.GetActorForwardVector`) (`self.Distance to move`))))
  (bind (_direction _actortolocation) (`Timeline|MoveToLocationTL`)
    (:`Update`
      (`self.K2_SetActorLocation` (`KismetMathLibrary.VLerp` (`self.SpawnWorkerLocation`) (`self.TargetWorkerLoc`) _actortolocation)))))

(fn `UserConstructionScript`)