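; BP_Boss is an office boss Blueprint that reports quest status when the first-person player character overlaps it.
; The overlap event loops over every row of the DT_OfficeQuests data table and reads each QuestCompleted flag.
; It prints each quest name with a Russian "done" or "not done" suffix, without changing any quest state.
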(event `self.ReceiveActorBeginOverlap`
  (params (OtherActor :type "Actor Object Reference"))
  (cast `/Game/FirstPerson/Blueprints/BP_FirstPersonCharacter` OtherActor)
  (bind _outrownames (`DataTableFunctionLibrary.GetDataTableRowNames` "/Game/Mgnoveniye/DT_OfficeQuests.DT_OfficeQuests"))
  (for _array_element _outrownames
    (bind _returnvalue (`|GetDataTableRow` "/Game/Mgnoveniye/DT_OfficeQuests.DT_OfficeQuests" _array_element)
      (:`then`
        (if (== (`.QuestCompleted_10_F108FC974C62CD40C0943AB20EBE77F6` (break `/Game/Mgnoveniye/BPS_OfficeQuests` _returnvalue)) true)
          (bind _returnvalue_2 (`KismetStringLibrary.Conv_NameToString` (break `/Game/Mgnoveniye/BPS_OfficeQuests` _returnvalue)))
          (`KismetSystemLibrary.PrintString` (`KismetStringLibrary.Concat_StrStr` _returnvalue_2 "выполнил"))
          (else
            (`KismetSystemLibrary.PrintString` (`KismetStringLibrary.Concat_StrStr` _returnvalue_2 "не выполнил"))))))))

(fn `UserConstructionScript`)