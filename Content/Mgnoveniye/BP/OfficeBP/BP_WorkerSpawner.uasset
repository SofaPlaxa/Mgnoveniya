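; BP_WorkerSpawner spawns coworker quest NPCs one after another during the player's office workday.
; Tick starts the workday when the player character's PlayerWorking flag is set, then spawns again whenever PlayerFinishedTalking is raised, clearing that flag.
; Each spawn begins the NPC's office behavior and increments the done count; once it exceeds today's quota, the next request clears PlayerWorking.
; WorkDayStart is never reset here.
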(event `StartWorkerSpawn`
  (if (>= (`self.OfficeWorkersToday`) (`self.OfficeWorkersDone`))
    (bind _returnvalue (`|SpawnActorFromClass` "/Game/Mgnoveniye/BP/OfficeBP/OfficeActors/NPCQuest_Coworker.NPCQuest_Coworker_C" (`KismetMathLibrary.MakeTransform` (`SceneComponent.K2_GetComponentLocation` (`self.DefaultSceneRoot`))) "Undefined" "MultiplyWithRoot" null (`GameplayStatics.GetPlayerCharacter` 0)))
    (`/Game/Mgnoveniye/BP/OfficeBP/OfficeActors/NPCQuest_Coworker.BeginOfficeWorker` _returnvalue)
    (`KismetSystemLibrary.PrintString` (`KismetSystemLibrary.GetDisplayName` _returnvalue))
    (bind _result (`/Engine/EditorBlueprintResources/StandardMacros.IncrementInt` (`self.OfficeWorkersDone`))
      (:`  `
        (set `self.OfficeWorkersDone` _result)))
    (else
      (bind _asbp_first_person_character (cast `/Game/FirstPerson/Blueprints/BP_FirstPersonCharacter` (`GameplayStatics.GetPlayerCharacter` 0)))
      (set `/Game/FirstPerson/Blueprints/BP_FirstPersonCharacter.PlayerWorking` false _asbp_first_person_character))))

(event `self.ReceiveTick`
  (params (DeltaSeconds :type "Float (single-precision)"))
  (if (`self.WorkDayStart`)
    (bind _asbp_first_person_character (cast `/Game/FirstPerson/Blueprints/BP_FirstPersonCharacter` (`GameplayStatics.GetPlayerCharacter` 0)))
    (if (`/Game/FirstPerson/Blueprints/BP_FirstPersonCharacter.PlayerFinishedTalking` _asbp_first_person_character)
      (`self.StartWorkerSpawn`)
      (set `/Game/FirstPerson/Blueprints/BP_FirstPersonCharacter.PlayerFinishedTalking` false _asbp_first_person_character))
    (else
      (bind _asbp_first_person_character_2 (cast `/Game/FirstPerson/Blueprints/BP_FirstPersonCharacter` (`GameplayStatics.GetPlayerCharacter` 0)))
      (if (`/Game/FirstPerson/Blueprints/BP_FirstPersonCharacter.PlayerWorking` _asbp_first_person_character_2)
        (set `self.WorkDayStart` true)
        (`self.StartWorkerSpawn`)))))

(fn `UserConstructionScript`)