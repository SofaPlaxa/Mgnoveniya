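; BP_BaseItem is a base interactable item whose construction script applies a configurable mesh and scales it by the inspection scale.
; On interaction with Inspect enabled, it spawns a BP_InspectItem far from the world origin.
; It passes that actor the inspection rotation, scale, mesh, name, description and interactor.
; With Inspect disabled it only prints a pick-up placeholder; BeginPlay caches a player character reference.
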(event `self.ReceiveBeginPlay`
  (bind _asbp_first_person_character (cast `/Game/FirstPerson/Blueprints/BP_FirstPersonCharacter` (`GameplayStatics.GetPlayerCharacter` 0)))
  (set `self.BP_PlayerRef` _asbp_first_person_character))

(event `/Game/Mgnoveniye/BP/DialogueSys/BPI_InteractInterface.InteractWithItem`
  (params (Interactor :type "/Game/FirstPerson/Blueprints/BP_FirstPersonCharacter Object Reference"))
  (if (`self.Inspect?`)
    (bind _returnvalue (`|SpawnActorFromClass` "/Game/Mgnoveniye/BP/ItemInspect/BP_InspectItem.BP_InspectItem_C" (`KismetMathLibrary.MakeTransform` (100000000.0 0.0 0.0)) "Undefined" "MultiplyWithRoot" null null))
    (`/Game/Mgnoveniye/BP/ItemInspect/BP_InspectItem.SetInspectRotation` _returnvalue (`self.ItemInspectionRotation`))
    (`/Game/Mgnoveniye/BP/ItemInspect/BP_InspectItem.SetInspectScale` _returnvalue (`self.ItemInspectionScale`))
    (message `/Game/Mgnoveniye/BP/DialogueSys/BPI_InteractInterface.Inspect` _returnvalue Interactor (`StaticMeshComponent.StaticMesh` (`self.StaticMesh`)) (`self.ItemName`) (`self.ItemDescription`))
    (else
      (`KismetSystemLibrary.PrintString` "pick up"))))

(fn `UserConstructionScript`
  (bind _staticmesh (`self.StaticMesh`))
  (`|ExecutionSequence`
    (:`then_0`
      (`StaticMeshComponent.SetStaticMesh` (`self.StaticMesh`) (`self.ItemMesh`))
      (`SceneComponent.K2_SetWorldTransform` _staticmesh (`KismetMathLibrary.MakeTransform` (`SceneComponent.K2_GetComponentLocation` _staticmesh) (`SceneComponent.K2_GetComponentRotation` _staticmesh) (`self.ItemInspectionScale`)) false false))))