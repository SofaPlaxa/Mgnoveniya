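; Item inspection actor that shows a given mesh with name and description in a WB_InspectItem widget.
; Inspect moves input from the player character to this actor, and callers can set the mesh's rotation and scale.
; Left-drag rotates the item, right-click resets rotation and zoom, and the wheel zooms by clamping the SceneCapture2D field of view.
; IA_Interact returns input to the character, removes the widget and destroys the actor.
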(event `/Game/Mgnoveniye/BP/DialogueSys/BPI_InteractInterface.Inspect`
  (params (Character :type "/Game/FirstPerson/Blueprints/BP_FirstPersonCharacter Object Reference") (InspectedItem :type "StaticMesh Object Reference") (ItemName :type Text) (ItemDescription :type Text))
  (bind _returnvalue (`GameplayStatics.GetPlayerController` 0))
  (set `self.PlayerCharacterRef` Character)
  (`StaticMeshComponent.SetStaticMesh` (`self.Item`) InspectedItem)
  (bind _returnvalue_2 (`|CreateWidget` "/Game/Mgnoveniye/BP/ItemInspect/WB_InspectItem.WB_InspectItem_C" null ItemName ItemDescription))
  (bind _output_get (set `self.InspectWRef` _returnvalue_2))
  (`UserWidget.AddToViewport` _output_get 0)
  (`self.DisableInput` (`self.PlayerCharacterRef`) _returnvalue)
  (`self.EnableInput` _returnvalue))

(event `EnhancedInput|/Game/FirstPerson/Input/Actions/IA_Interact`
  (params (ActionValue :type Boolean) (ElapsedSeconds :type "Float (double-precision)") (TriggeredSeconds :type "Float (double-precision)") (InputAction :type "InputAction Object Reference" :default "/Game/FirstPerson/Input/Actions/IA_Interact.IA_Interact"))
  (bind _returnvalue (`GameplayStatics.GetPlayerController` 0))
  (bind _inspectwref (`self.InspectWRef`))
  (:`Started`
    (`self.DisableInput` _returnvalue)
    (`self.EnableInput` (`self.PlayerCharacterRef`) _returnvalue)
    (`/Engine/EditorBlueprintResources/StandardMacros.IsValid` _inspectwref
      (:`Is Valid`
        (`Widget.RemoveFromParent` _inspectwref)
        (set `self.InspectWRef` null)
        (`self.K2_DestroyActor`)))))

(event `SetInspectRotation`
  (params (ItemRotation :type "Rotator Structure"))
  (bind _item (`self.Item`))
  (bind (_returnvalue_location _returnvalue_rotation _returnvalue_scale) (`KismetMathLibrary.BreakTransform` (`SceneComponent.K2_GetComponentToWorld` _item)))
  ; Set rotation d
  (bind _output_get (set `self.Initial Item Rotation` ItemRotation))
  (`SceneComponent.K2_SetWorldTransform` _item (`KismetMathLibrary.MakeTransform` _returnvalue_location _output_get _returnvalue_scale) false false))

(event `SetInspectScale`
  (params (InspectionScale :type "Vector Structure"))
  (bind _item (`self.Item`))
  (bind (_returnvalue_location _returnvalue_rotation) (`KismetMathLibrary.BreakTransform` (`SceneComponent.K2_GetComponentToWorld` _item)))
  ; Set inspection scale d
  (`SceneComponent.K2_SetWorldTransform` _item (`KismetMathLibrary.MakeTransform` _returnvalue_location _returnvalue_rotation InspectionScale) false false))

(event `Key|LeftMouseButton`
  (params (Key :type "Key Structure"))
  ; Rotate when lclick
  (:`Pressed`
    (set `self.Rotate?` true))
  (:`Released`
    (set `self.Rotate?` false)))

(event `Key|RightMouseButton`
  (params (Key :type "Key Structure"))
  ; ResetTransform
  (:`Pressed`
    (`SceneComponent.K2_SetWorldRotation` (`self.Item`) (`self.Initial Item Rotation`) false false)
    (set `SceneCaptureComponent2D.FOVAngle` 50.0 (`self.SceneCaptureComponent2D`))))

(event `InputAxisKey|MouseX`
  (params (AxisValue :type "Float (single-precision)"))
  ; Set mouse movement horiz
  (if (`self.Rotate?`)
    (`SceneComponent.K2_SetWorldRotation` (`self.Item`) (`KismetMathLibrary.ComposeRotators` (`SceneComponent.K2_GetComponentRotation` (`self.Item`)) (`KismetMathLibrary.MakeRotator` 0.0 0.0 (* AxisValue -3.0))) false false)))

(event `InputAxisKey|MouseY`
  (params (AxisValue :type "Float (single-precision)"))
  ; Set mouse movement vert
  (if (`self.Rotate?`)
    (`SceneComponent.K2_SetWorldRotation` (`self.Item`) (`KismetMathLibrary.ComposeRotators` (`SceneComponent.K2_GetComponentRotation` (`self.Item`)) (`KismetMathLibrary.MakeRotator` 0.0 (* AxisValue -3.0))) false false)))

(event `Key|MouseScrollUp`
  (params (Key :type "Key Structure"))
  (bind _scenecapturecomponent2d (`self.SceneCaptureComponent2D`))
  ; ZoomIn
  (:`Pressed`
    (set `SceneCaptureComponent2D.FOVAngle` (`KismetMathLibrary.FClamp` (- (`SceneCaptureComponent2D.FOVAngle` _scenecapturecomponent2d) 1.0) 30.0 80.0) _scenecapturecomponent2d)))

(event `Key|MouseScrollDown`
  (params (Key :type "Key Structure"))
  (bind _scenecapturecomponent2d (`self.SceneCaptureComponent2D`))
  ; Zoom out
  (:`Pressed`
    (set `SceneCaptureComponent2D.FOVAngle` (`KismetMathLibrary.FClamp` (+ (`SceneCaptureComponent2D.FOVAngle` _scenecapturecomponent2d) 1.0) 30.0 80.0) _scenecapturecomponent2d)))

(fn `InteractWithItem`
  (params (Interactor :type "Character Object Reference"))
  (returns (`DidInteract?` :type Boolean))
  (return false))

(fn `UserConstructionScript`)