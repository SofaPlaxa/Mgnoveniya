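; Test dialogue NPC actor drawn as an eight-direction Paper2D billboard that the player can talk to.
; Each tick, the player's angle from its forward vector, signed by the right vector, selects the flipbook rotation and idle flipbook in 45-degree sectors.
; Each Talk call flags the first-person character as in dialogue and shows the next Dialogue1 line in WB_DialogueWindow, removing the widget and clearing the flag after the last.
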(event `self.ReceiveTick`
  (params (DeltaSeconds :type "Float (single-precision)"))
  (bind _degrees (`self.Degrees`))
  (bind _degrees_2 (`self.Degrees`))
  (bind _returnvalue (`KismetMathLibrary.Normal` (- (`self.K2_GetActorLocation` (`GameplayStatics.GetPlayerCharacter` 0)) (`self.K2_GetActorLocation`))))
  ;[1 1 1] Billboard 4D
  (set `self.Degrees` (`KismetMathLibrary.DegAcos` (`KismetMathLibrary.Dot_VectorVector` (`self.GetActorForwardVector`) _returnvalue)))
  (if (< (`KismetMathLibrary.Dot_VectorVector` _returnvalue (`self.GetActorRightVector`)) 0.0)
    (`/Engine/EditorBlueprintResources/StandardMacros.CompareFloat` _degrees_2 180.0
      (:`>`
        (`SceneComponent.K2_SetRelativeRotation` (`self.PaperFlipbook`) (struct :`Yaw` -90.0) false false :!label _label)
        (`PaperFlipbookComponent.SetFlipbook` (`self.PaperFlipbook`) (`|GetArrayItem` (`self.Fbooks_Idle`))))
      (:`==`
        (goto _label))
      (:`<`
        (`/Engine/EditorBlueprintResources/StandardMacros.CompareFloat` _degrees_2 135.0
          (:`>`
            (`SceneComponent.K2_SetRelativeRotation` (`self.PaperFlipbook`) (struct :`Yaw` 135.0) false false :!label _label_2)
            (`PaperFlipbookComponent.SetFlipbook` (`self.PaperFlipbook`) (`|GetArrayItem` (`self.Fbooks_Idle`) 3)))
          (:`==`
            (goto _label_2))
          (:`<`
            (`/Engine/EditorBlueprintResources/StandardMacros.CompareFloat` _degrees_2 90.0
              (:`>`
                (`SceneComponent.K2_SetRelativeRotation` (`self.PaperFlipbook`) (struct :`Yaw` 180.0) false false :!label _label_3)
                (`PaperFlipbookComponent.SetFlipbook` (`self.PaperFlipbook`) (`|GetArrayItem` (`self.Fbooks_Idle`) 2)))
              (:`==`
                (goto _label_3))
              (:`<`
                (`/Engine/EditorBlueprintResources/StandardMacros.CompareFloat` _degrees_2 45.0
                  (:`>`
                    _)
                  (:`==`
                    _)
                  (:`<`
                    (goto _label)))
                (`SceneComponent.K2_SetRelativeRotation` (`self.PaperFlipbook`) (struct :`Yaw` -135.0) false false)
                (`PaperFlipbookComponent.SetFlipbook` (`self.PaperFlipbook`) (`|GetArrayItem` (`self.Fbooks_Idle`) 1))))))))
    (else
      (`/Engine/EditorBlueprintResources/StandardMacros.CompareFloat` _degrees 180.0
        (:`>`
          (`SceneComponent.K2_SetRelativeRotation` (`self.PaperFlipbook`) (struct :`Yaw` -45.0) false false :!label _label_4)
          (`PaperFlipbookComponent.SetFlipbook` (`self.PaperFlipbook`) (`|GetArrayItem` (`self.Fbooks_Idle`) 7)))
        (:`==`
          (goto _label_4))
        (:`<`
          (`/Engine/EditorBlueprintResources/StandardMacros.CompareFloat` _degrees 135.0
            (:`>`
              (`SceneComponent.K2_SetRelativeRotation` (`self.PaperFlipbook`) (struct :`Yaw` 90.0) false false :!label _label_5)
              (`PaperFlipbookComponent.SetFlipbook` (`self.PaperFlipbook`) (`|GetArrayItem` (`self.Fbooks_Idle`) 4)))
            (:`==`
              (goto _label_5))
            (:`<`
              (`/Engine/EditorBlueprintResources/StandardMacros.CompareFloat` _degrees 90.0
                (:`>`
                  (`SceneComponent.K2_SetRelativeRotation` (`self.PaperFlipbook`) (struct :`Yaw` 45.0) false false :!label _label_6)
                  (`PaperFlipbookComponent.SetFlipbook` (`self.PaperFlipbook`) (`|GetArrayItem` (`self.Fbooks_Idle`) 5)))
                (:`==`
                  (goto _label_6))
                (:`<`
                  (`/Engine/EditorBlueprintResources/StandardMacros.CompareFloat` _degrees 45.0
                    (:`>`
                      _)
                    (:`==`
                      _)
                    (:`<`
                      (goto _label_4)))
                  (`SceneComponent.K2_SetRelativeRotation` :`self` (`self.PaperFlipbook`))
                  (`PaperFlipbookComponent.SetFlipbook` (`self.PaperFlipbook`) (`|GetArrayItem` (`self.Fbooks_Idle`) 6)))))))))))

(event `/Game/Mgnoveniye/Art/DialogueSystem/BPI_DialogueTest.Talk`
  (bind _asbp_first_person_character (cast `/Game/FirstPerson/Blueprints/BP_FirstPersonCharacter` (`GameplayStatics.GetPlayerCharacter` 0)))
  (bind _output_get (set `/Game/FirstPerson/Blueprints/BP_FirstPersonCharacter.InDialogue` true _asbp_first_person_character))
  (`KismetSystemLibrary.PrintString` (`KismetStringLibrary.Conv_BoolToString` _output_get))
  (`/Engine/EditorBlueprintResources/StandardMacros.IncrementInt` (`self.TalkIndex`)
    (:`  `
      (if (< (`self.TalkIndex`) (`KismetArrayLibrary.Array_Length` (`self.Dialogue1`)))
        (`self.UI`
          (:`then`
            _)
          (:`else`
            (bind _returnvalue (`|CreateWidget` "/Game/Mgnoveniye/Art/DialogueSystem/WB_DialogueWindow.WB_DialogueWindow_C" (`GameplayStatics.GetPlayerController` 0)))
            (bind _output_get_2 (set `self.UI` _returnvalue))
            (`UserWidget.AddToViewport` _output_get_2 0)))
        (`TextBlock.SetText` (`/Game/Mgnoveniye/Art/DialogueSystem/WB_DialogueWindow.TalkText` (`self.UI`)) (`KismetTextLibrary.Conv_StringToText` (`|GetArrayItem` (`self.Dialogue1`) (`self.TalkIndex`))))
        (else
          (`Widget.RemoveFromParent` (`self.UI`))
          (set `self.TalkIndex` -1)
          (set `self.UI` null)
          (bind _asbp_first_person_character_2 (cast `/Game/FirstPerson/Blueprints/BP_FirstPersonCharacter` (`GameplayStatics.GetPlayerCharacter` 0)))
          (bind _output_get_3 (set `/Game/FirstPerson/Blueprints/BP_FirstPersonCharacter.InDialogue` false _asbp_first_person_character_2))
          (`KismetSystemLibrary.PrintString` (`KismetStringLibrary.Conv_BoolToString` _output_get_3)))))))

(fn `UserConstructionScript`)