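; Base actor component for branching conversations, which opens a WB_Dialogue widget and notifies its owner when the conversation closes.
; Dialogue is an empty hook, re-run from the start each time an option is selected.
; AddDialogue replays stored choices from the DialogueProgress map by step index, or shows an unanswered line and sets the speaker's emote.
; Progress can be cleared, rolled back several steps, or reset by switching dialogue tree.
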(fn `AddDialogue`
  (params (SpeakerName :type Text) (DialogueText :type Text) (OptionsText :type "Array of Text") (NewFace :type Integer))
  (returns (State :type "/Game/Mgnoveniye/BP/DialogueSys/Enum_DialogueState Enum") (OptionIndex :type Integer))
  (bind (_value _returnvalue) (`BlueprintMapLibrary.Map_Find` (`self.DialogueProgress`) (`self.DialogueIndex`)))
  (`/Engine/EditorBlueprintResources/StandardMacros.IncrementInt` (`self.DialogueIndex`)
    (:`  `
      (if _returnvalue
        (return "NewEnumerator0" _value)
        (else
          (`/Game/Mgnoveniye/UI/DialogueUI/WB_Dialogue.UpdateDialogueText` (`self.DialogueWidget`) (`self.DialogueIndex`) (`local.SpeakerName`) (`local.DialogueText`) (`local.OptionsText`))
          (set `self.CurrentEmote` NewFace)
          (return "NewEnumerator1" 0))))))

(fn `ClearDialogueProgress`
  (`BlueprintMapLibrary.Map_Clear` (`self.DialogueProgress`)))

(fn `CloseConversation`
  (`Widget.RemoveFromParent` (`self.DialogueWidget`))
  (message `/Game/Mgnoveniye/BP/DialogueSys/BPI_InteractInterface.ConversationClosed` (`self.GetOwner`)))

(fn `Dialogue`)

(fn `OpenConversation`
  (bind _returnvalue (`|CreateWidget` "/Game/Mgnoveniye/UI/DialogueUI/WB_Dialogue.WB_Dialogue_C" null self))
  (bind _output_get (set `self.DialogueWidget` _returnvalue))
  (`UserWidget.AddToViewport` _output_get 0)
  (`self.ProgressDialogue`))

(fn `ProgressDialogue`
  (set `self.DialogueIndex` -1)
  (`self.Dialogue`))

(fn `RemoveDialogueProgress`
  (params (ProgressSteps :type Integer))
  (for _index (range (+ ProgressSteps 1))
    (`BlueprintMapLibrary.Map_Remove` (`self.DialogueProgress`) (- (`self.DialogueIndex`) _index))))

(fn `SetDialogueTreeIndex`
  (params (DialogueTreeIndex :type Integer))
  (set `self.DialogueTreeIndex` DialogueTreeIndex)
  (`self.ClearDialogueProgress`))

(fn `UpdateEmote`
  (set `self.CurrentEmote` 0))

(fn `UpdateSelectedOption`
  (params (ProgressIndex :type "Integer (by ref)") (OptionIndex :type "Integer (by ref)"))
  (`BlueprintMapLibrary.Map_Add` (`self.DialogueProgress`) ProgressIndex OptionIndex)
  (`self.ProgressDialogue`))