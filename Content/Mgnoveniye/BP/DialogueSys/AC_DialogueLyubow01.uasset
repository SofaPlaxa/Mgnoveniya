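; Dialogue component for the NPC Lyubov Sergeevna, an office coworker who chats with Oleg about paperwork and grumbles about the new employee Mark.
; The Dialogue function extends its parent and branches on DialogueTreeIndex, chaining AddDialogue calls that advance on Pass Through, with player choices not altering the flow.
; The first tree plays the full exchange, then switches to the second, which shows one of two random short lines, clears progress and closes the conversation.
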(fn `Dialogue`
  (`parent.Dialogue`)
  (switch `int` (`self.DialogueTreeIndex`)
    (:`0`
      (bind (_state _optionindex) (`self.AddDialogue` "Любовь Сергеевна" "О! Олег, ты отправил мне те бумаги, что я вчера просила?" (`|MakeArray` "Доброе утро, Любовь Сергеевна. Отправил, конечно. На почте проверьте" :!type "Text")))
      (switch `/Game/Mgnoveniye/BP/DialogueSys/Enum_DialogueState` _state
        (:`NewEnumerator0`
          (switch `int` _optionindex
            (:`0`
              _)
            (:`1`
              _))
          (bind (_state_2 _optionindex_2) (`self.AddDialogue` "Любовь Сергеевна" "На почте, говорит… Ага, у нас всё на почте, а бумаги потом я ищи по всем флэшкам!  \nМолодёжь пошла электронная, а папки всё равно я таскаю." (`|MakeArray` "Если хотите, могу помочь с переносом…" "..." :!type "Text")))
          (switch `/Game/Mgnoveniye/BP/DialogueSys/Enum_DialogueState` _state_2
            (:`NewEnumerator0`
              (switch `int` _optionindex_2
                (:`0`
                  _)
                (:`1`
                  _))
              (bind (_state_3 _optionindex_3) (`self.AddDialogue` "Любовь Сергеевна" "Ха! Я тебя скорее до третьего этажа донесу, чем ты меня разгрузишь. Ты работай лучше!" (`|MakeArray` "Мне не сложно, правда" "..." :!type "Text")))
              (switch `/Game/Mgnoveniye/BP/DialogueSys/Enum_DialogueState` _state_3
                (:`NewEnumerator0`
                  (switch `int` _optionindex_3
                    (:`0`
                      _)
                    (:`1`
                      _))
                  (bind (_state_4 _optionindex_4) (`self.AddDialogue` "Любовь Сергеевна" "А вон тот новый, с серёжкой в ухе, совсем бумагу не различает от пластика, пусть он займется" (`|MakeArray` "Это Марк. Он… старается" :!type "Text")))
                  (switch `/Game/Mgnoveniye/BP/DialogueSys/Enum_DialogueState` _state_4
                    (:`NewEnumerator0`
                      (switch `int` _optionindex_4
                        (:`0`
                          _)
                        (:`1`
                          _))
                      (bind _state_5 (`self.AddDialogue` "Любовь Сергеевна" "Пусть старается в другом месте! У нас тут не кружок хендмейда" (`|MakeArray` "..." :!type "Text")))
                      (switch `/Game/Mgnoveniye/BP/DialogueSys/Enum_DialogueState` _state_5
                        (:`NewEnumerator0`
                          (`self.SetDialogueTreeIndex` 1)
                          (`self.CloseConversation`))))))))))))
    (:`1`
      (bind _state_6 (`self.AddDialogue` "Любовь Сергеевна" (select `int` (`KismetMathLibrary.RandomIntegerInRange` 0 1) :`0` "М?" :`1` "Я к тебе еще загляну, нужна помощь с документами..." :!type "Text") (`|MakeArray` "уйти" :!type "Text")))
      (switch `/Game/Mgnoveniye/BP/DialogueSys/Enum_DialogueState` _state_6
        (:`NewEnumerator0`
          (`self.ClearDialogueProgress`)
          (`self.CloseConversation`))))))