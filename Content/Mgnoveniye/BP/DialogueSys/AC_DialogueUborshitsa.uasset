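; Dialogue component for the cleaning lady Надежда, who greets the player and grumbles about her freshly mopped floor.
; It overrides the parent's Dialogue function, chaining two AddDialogue lines with reply options through their Pass Through states.
; After the second line it sets the dialogue tree index to 1 and closes the conversation.
; The switches on tree index and first reply have empty branches, and the second reply choice does not alter the outcome.
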(fn `Dialogue`
  (`parent.Dialogue`)
  (switch `int` (`self.DialogueTreeIndex`)
    (:`0`
      _)
    (:`1`
      _))
  (bind (_state _optionindex) (`self.AddDialogue` "Надежда" "Ой, здравствуй, милый. Ты тут только не шлёпай по лужам, я только вымыла." (`|MakeArray` "Постараюсь" :!type "Text")))
  (switch `/Game/Mgnoveniye/BP/DialogueSys/Enum_DialogueState` _state
    (:`NewEnumerator0`
      (switch `int` _optionindex
        (:`0`
          _)
        (:`1`
          _))
      (bind _state_2 (`self.AddDialogue` "Надежда" "Постараюсь он говорит… А я потом старайся с этими разводами. Третий раз за утро, между прочим." (`|MakeArray` "Спасибо за ваш труд" "..." :!type "Text")))
      (switch `/Game/Mgnoveniye/BP/DialogueSys/Enum_DialogueState` _state_2
        (:`NewEnumerator0`
          (`self.SetDialogueTreeIndex` 1)
          (`self.CloseConversation`))))))