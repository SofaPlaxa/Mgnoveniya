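; Dialogue component for the woman with a dog NPC, scripting her Russian-language conversation about her touchy dog Bonya.
; Dialogue runs the parent, then switches on DialogueTreeIndex: the first tree chains AddDialogue calls on Pass Through, with reply choices that never branch.
; Its final AddDialogue is followed by setting index 1 and closing, without a state check.
; Tree 1 shows one of two random greetings, then clears progress and closes.
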(fn `Dialogue`
  (`parent.Dialogue`)
  (switch `int` (`self.DialogueTreeIndex`)
    (:`0`
      (bind (_state _optionindex) (`self.AddDialogue` "Женщина с собачкой" "Осторожнее! Вы едва не спугнули Боню. У него, между прочим, слабые нервы!" (`|MakeArray` "Прошу прощения, не заметил" "Мне жаль, не заметил" :!type "Text")))
      (switch `/Game/Mgnoveniye/BP/DialogueSys/Enum_DialogueState` _state
        (:`NewEnumerator0`
          (switch `int` _optionindex
            (:`0`
              _)
            (:`1`
              _))
          (bind (_state_2 _optionindex_2) (`self.AddDialogue` "Женщина с собачкой" "Конечно не заметили. Никто сейчас ничего не замечает. Все куда-то бегут. А Боня — чувствительная натура" (`|MakeArray` "..." :!type "Text")))
          (switch `/Game/Mgnoveniye/BP/DialogueSys/Enum_DialogueState` _state_2
            (:`NewEnumerator0`
              (switch `int` _optionindex_2
                (:`0`
                  _)
                (:`1`
                  _))
              (bind (_state_3 _optionindex_3) (`self.AddDialogue` "Боня" "ТЯФ!" (`|MakeArray` "Он… кажется, не в обмороке" "Выглядит бодрым" :!type "Text")))
              (switch `/Game/Mgnoveniye/BP/DialogueSys/Enum_DialogueState` _state_3
                (:`NewEnumerator0`
                  (switch `int` _optionindex_3
                    (:`0`
                      _)
                    (:`1`
                      _))
                  (bind (_state_4 _optionindex_4) (`self.AddDialogue` "Женщина с собачкой" "Это — демонстративное неодобрение. Он не одобряет ваш тон" (`|MakeArray` "..." :!type "Text")))
                  (switch `/Game/Mgnoveniye/BP/DialogueSys/Enum_DialogueState` _state_4
                    (:`NewEnumerator0`
                      (switch `int` _optionindex_4
                        (:`0`
                          _)
                        (:`1`
                          _))
                      (bind (_state_5 _optionindex_5) (`self.AddDialogue` "Женщина с собачкой" "Мужчины сейчас всё грубее. Раньше за мной машины останавливались…" (`|MakeArray` "Ваша пара — образец утончённого стиля" :!type "Text")))
                      (switch `/Game/Mgnoveniye/BP/DialogueSys/Enum_DialogueState` _state_5
                        (:`NewEnumerator0`
                          (switch `int` _optionindex_5
                            (:`0`
                              _)
                            (:`1`
                              _))
                          (bind (_state_6 _optionindex_6) (`self.AddDialogue` "Женщина с собачкой" "Ну, хоть кто-то заметил. Боня всегда требует стиль!" (`|MakeArray` "..." :!type "Text")))
                          (switch `/Game/Mgnoveniye/BP/DialogueSys/Enum_DialogueState` _state_6
                            (:`NewEnumerator0`
                              (switch `int` _optionindex_6
                                (:`0`
                                  _)
                                (:`1`
                                  _))
                              (`self.AddDialogue` "Женщина с собачкой" "И всё-таки — не спешите так. От этого появляются морщины." (`|MakeArray` "..." :!type "Text"))
                              (`self.SetDialogueTreeIndex` 1)
                              (`self.CloseConversation`))))))))))))))
    (:`1`
      (bind _state_7 (`self.AddDialogue` "Женщина с собачкой" (select `int` (`KismetMathLibrary.RandomIntegerInRange` 0 1) :`0` "Боня сразу узнал вашу походку" :`1` "Ваши комплименты — лучшее начало дня" :!type "Text") (`|MakeArray` "уйти" :!type "Text")))
      (switch `/Game/Mgnoveniye/BP/DialogueSys/Enum_DialogueState` _state_7
        (:`NewEnumerator0`
          (`self.ClearDialogueProgress`)
          (`self.CloseConversation`))))))