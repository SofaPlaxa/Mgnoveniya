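; Dialogue component for an elderly woman NPC ("Бабка"), holding her Russian small talk with the player about the bus and work.
; It overrides Dialogue, calls the parent, then switches on DialogueTreeIndex to chain AddDialogue steps gated on their Pass Through state.
; Tree 0 is a linear first conversation whose choices do not branch, ending by switching to tree 1.
; Tree 1 gives one of two random send-off lines, then clears progress and closes.
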(fn `Dialogue`
  (`parent.Dialogue`)
  (switch `int` (`self.DialogueTreeIndex`)
    (:`0`
      (bind (_state _optionindex) (`self.AddDialogue` "Пожилая женщина" "Ой, здравствуй, милок. Ты, случаем, не знаешь, автобус уже уходил?" (`|MakeArray` "Не знаю" "По расписанию — через три минуты" :!type "Text")))
      (switch `/Game/Mgnoveniye/BP/DialogueSys/Enum_DialogueState` _state
        (:`NewEnumerator0`
          (switch `int` _optionindex
            (:`0`
              _)
            (:`1`
              _))
          (bind (_state_2 _optionindex_2) (`self.AddDialogue` "Бабка" "Ох, ну и хорошо. А то я всё боюсь опоздать, ноги уже не те." (`|MakeArray` "..." :!type "Text")))
          (switch `/Game/Mgnoveniye/BP/DialogueSys/Enum_DialogueState` _state_2
            (:`NewEnumerator0`
              (switch `int` _optionindex_2
                (:`0`
                  _)
                (:`1`
                  _))
              (bind (_state_3 _optionindex_3) (`self.AddDialogue` "Бабка" "Ты на работу, да?" (`|MakeArray` "Да. Обычно тоже этим маршрутом" "Куда же еще в такую рань" :!type "Text")))
              (switch `/Game/Mgnoveniye/BP/DialogueSys/Enum_DialogueState` _state_3
                (:`NewEnumerator0`
                  (switch `int` _optionindex_3
                    (:`0`
                      _)
                    (:`1`
                      _))
                  (bind (_state_4 _optionindex_4) (`self.AddDialogue` "Бабка" "Вижу по глазам — серьёзный ты, ответственный. Прям как мой Витя был. Всё бегом, всё по часам…" (`|MakeArray` "Привычка. Без порядка тяжело" "..." :!type "Text")))
                  (switch `/Game/Mgnoveniye/BP/DialogueSys/Enum_DialogueState` _state_4
                    (:`NewEnumerator0`
                      (switch `int` _optionindex_4
                        (:`0`
                          _)
                        (:`1`
                          _))
                      (`self.AddDialogue` "Бабка" "Береги себя, сынок. Люди теперь такие суетные… А доброта — она, знаешь, не теряет срока годности" (`|MakeArray` "Спасибо. Хорошего вам дня" :!type "Text"))
                      (`self.SetDialogueTreeIndex` 1)
                      (`self.CloseConversation`))))))))))
    (:`1`
      (bind _state_5 (`self.AddDialogue` "Бабка" (select `int` (`KismetMathLibrary.RandomIntegerInRange` 0 1) :`0` "Иди-иди, не опоздай, а то начальство ругаться будет!" :`1` "Ты как мой Виктор… всё в делах, всё спешит..." :!type "Text") (`|MakeArray` "уйти" :!type "Text")))
      (switch `/Game/Mgnoveniye/BP/DialogueSys/Enum_DialogueState` _state_5
        (:`NewEnumerator0`
          (`self.ClearDialogueProgress`)
          (`self.CloseConversation`))))))