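; Dialogue component for the character Olya, defining her branching conversation with the player in an override of the parent's Dialogue function.
; DialogueTreeIndex picks the tree, and nested AddDialogue calls branch on the chosen option once their state passes through.
; Completing the question branch advances to tree 1, which gives a random one-liner on later talks.
; Other endings clear or roll back dialogue progress before closing the conversation.
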(fn `Dialogue`
  (`parent.Dialogue`)
  (switch `int` (`self.DialogueTreeIndex`)
    (:`0`
      (bind (_state _optionindex) (`self.AddDialogue` "Olya" "hi! how's your day?" (`|MakeArray` "it's fine" "trash" :!type "Text")))
      (switch `/Game/Mgnoveniye/BP/DialogueSys/Enum_DialogueState` _state
        (:`NewEnumerator0`
          (switch `int` _optionindex
            (:`0`
              (bind (_state_2 _optionindex_2) (`self.AddDialogue` "Olya" "nice! may i ask you a question?" (`|MakeArray` "go ahead" "nah" :!type "Text")))
              (switch `/Game/Mgnoveniye/BP/DialogueSys/Enum_DialogueState` _state_2
                (:`NewEnumerator0`
                  (switch `int` _optionindex_2
                    (:`0`
                      (bind _state_3 (`self.AddDialogue` "Olya" "why u so grumpy?" (`|MakeArray` "damn." "i'm not" :!type "Text")))
                      (switch `/Game/Mgnoveniye/BP/DialogueSys/Enum_DialogueState` _state_3
                        (:`NewEnumerator0`
                          (`self.SetDialogueTreeIndex` 1)
                          (`self.CloseConversation`))))
                    (:`1`
                      (bind _state_4 (`self.AddDialogue` "Olya" "u big meany" (`|MakeArray` "continue" :!type "Text")))
                      (switch `/Game/Mgnoveniye/BP/DialogueSys/Enum_DialogueState` _state_4
                        (:`NewEnumerator0`
                          (`self.RemoveDialogueProgress` 2)
                          (`self.CloseConversation`))))))))
            (:`1`
              (bind _state_5 (`self.AddDialogue` "Olya" "i'm sad now" (`|MakeArray` "continue" :!type "Text")))
              (switch `/Game/Mgnoveniye/BP/DialogueSys/Enum_DialogueState` _state_5
                (:`NewEnumerator0`
                  (`self.ClearDialogueProgress`)
                  (`self.CloseConversation`))))))))
    (:`1`
      (bind _state_6 (`self.AddDialogue` "Olya" (select `int` (`KismetMathLibrary.RandomIntegerInRange` 0 1) :`0` "i was joking" :`1` "heehehhehehe" :!type "Text") (`|MakeArray` "continue" :!type "Text")))
      (switch `/Game/Mgnoveniye/BP/DialogueSys/Enum_DialogueState` _state_6
        (:`NewEnumerator0`
          (`self.ClearDialogueProgress`)
          (`self.CloseConversation`))))))