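; Dialogue component for Anatoly Grigoryevich's morning briefing with Oleg, covering a meeting, trip bookings and a client anniversary.
; Overrides Dialogue as nested AddDialogue calls branched on DialogueTreeIndex, with one reply per line and face changes.
; Sequence branches play a writing sound and add items to WB_Notebook mid-conversation.
; The ending advances the index and shows WB_ThankYou; later talks give a random one-liner labelled as Mark (Марк).
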(fn `Dialogue`
  (`parent.Dialogue`)
  (switch `int` (`self.DialogueTreeIndex`)
    (:`0`
      (bind (_state _optionindex) (`self.AddDialogue` "Анатолий Григорьевич" "Олег, доброе утро. Отдел маркетинга запрашивал встречу на сегодня." (`|MakeArray` "Доброе утро. Да, видел. На какое время назначим?" :!type "Text") 1))
      (switch `/Game/Mgnoveniye/BP/DialogueSys/Enum_DialogueState` _state
        (:`NewEnumerator0`
          (switch `int` _optionindex
            (:`0`
              (bind (_state_2 _optionindex_2) (`self.AddDialogue` "Анатолий Григорьевич" "Давай на семь вечера, если окно свободно." (`|MakeArray` "Семь подходит. В вашем кабинете или в конференц-зале?" :!type "Text") 5))
              (switch `/Game/Mgnoveniye/BP/DialogueSys/Enum_DialogueState` _state_2
                (:`NewEnumerator0`
                  (switch `int` _optionindex_2
                    (:`0`
                      (bind (_state_3 _optionindex_3) (`self.AddDialogue` "Анатолий Григорьевич" "В зале удобнее. Кстати, в субботу лечу в Питер, не забудь." (`|MakeArray` " Уже делаю. Какие пожелания по бронированию?" :!type "Text")))
                      (switch `/Game/Mgnoveniye/BP/DialogueSys/Enum_DialogueState` _state_3
                        (:`NewEnumerator0`
                          (switch `int` _optionindex_3
                            (:`0`
                              (bind (_state_4 _optionindex_4) (`self.AddDialogue` "Анатолий Григорьевич" "Лучше утренний рейс, часов в девять. И забронируй столик в «Кристалле» на пятерых на семь вечера. Плюс номер в гостинице на одного." (`|MakeArray` "Сегодня все улажу, билеты будут у вас на столе . Кстати, в среду юбилей у НПО «Салфеточный союз». Напомнить вам за день?" :!type "Text") 3))
                              (`|ExecutionSequence`
                                (:`then_0`
                                  (switch `/Game/Mgnoveniye/BP/DialogueSys/Enum_DialogueState` _state_4
                                    (:`NewEnumerator0`
                                      (switch `int` _optionindex_4
                                        (:`0`
                                          (bind (_state_5 _optionindex_5) (`self.AddDialogue` "Анатолий Григорьевич" "Батюшки! Как быстро растут чужие фирмы. Неужели уже пятнадцать лет?" (`|MakeArray` "Да, пятнадцать." :!type "Text") 2))
                                          (`|ExecutionSequence`
                                            (:`then_0`
                                              (switch `/Game/Mgnoveniye/BP/DialogueSys/Enum_DialogueState` _state_5
                                                (:`NewEnumerator0`
                                                  (switch `int` _optionindex_5
                                                    (:`0`
                                                      (bind (_state_6 _optionindex_6) (`self.AddDialogue` "Анатолий Григорьевич" "Потрясающе. Молодцы ребята! Хорошо, с подарком разберусь лично. Что-то еще?" (`|MakeArray` " Пока все." :!type "Text") 4))
                                                      (`|ExecutionSequence`
                                                        (:`then_0`
                                                          (switch `/Game/Mgnoveniye/BP/DialogueSys/Enum_DialogueState` _state_6
                                                            (:`NewEnumerator0`
                                                              (switch `int` _optionindex_6
                                                                (:`0`
                                                                  (bind _state_7 (`self.AddDialogue` "Анатолий Григорьевич" " Понял тебя. Тогда за работу! " (`|MakeArray` "Далее" :!type "Text")))
                                                                  (switch `/Game/Mgnoveniye/BP/DialogueSys/Enum_DialogueState` _state_7
                                                                    (:`NewEnumerator0`
                                                                      (`self.SetDialogueTreeIndex` 1)
                                                                      (`self.CloseConversation`)
                                                                      (bind _returnvalue (`|CreateWidget` "/Game/Mgnoveniye/UI/Loading/WB_ThankYou.WB_ThankYou_C" (`GameplayStatics.GetPlayerController` 0)))
                                                                      (`UserWidget.AddToViewport` _returnvalue 0))))))))
                                                        (:`then_1`
                                                          (`GameplayStatics.PlaySound2D` "/Game/Mgnoveniye/SFX/NewWAWSound/InteractWithWorld/SC_WriteNote.SC_WriteNote" 1.0 1.0 0.0 null null)
                                                          (bind _foundwidgets (`WidgetBlueprintLibrary.GetAllWidgetsOfClass` "/Game/Mgnoveniye/UI/OfficeTask/WB_Notebook.WB_Notebook_C"))
                                                          (bind _output (`|GetArrayItem` _foundwidgets))
                                                          (`/Engine/EditorBlueprintResources/StandardMacros.IsValid` _output
                                                            (:`Is Valid`
                                                              (bind _output_get (set `/Game/Mgnoveniye/UI/OfficeTask/WB_Notebook.NoteItemIndex` 10 _output))
                                                              (`/Game/Mgnoveniye/UI/OfficeTask/WB_Notebook.AddNoteItem` _output _output_get))))))))))
                                            (:`then_1`
                                              (`GameplayStatics.PlaySound2D` "/Game/Mgnoveniye/SFX/NewWAWSound/InteractWithWorld/SC_WriteNote.SC_WriteNote" 1.0 1.0 0.0 null null)
                                              (bind _foundwidgets_2 (`WidgetBlueprintLibrary.GetAllWidgetsOfClass` "/Game/Mgnoveniye/UI/OfficeTask/WB_Notebook.WB_Notebook_C"))
                                              (bind _output_2 (`|GetArrayItem` _foundwidgets_2))
                                              (`/Engine/EditorBlueprintResources/StandardMacros.IsValid` _output_2
                                                (:`Is Valid`
                                                  (bind _output_get_2 (set `/Game/Mgnoveniye/UI/OfficeTask/WB_Notebook.NoteItemIndex` 8 _output_2))
                                                  (`/Game/Mgnoveniye/UI/OfficeTask/WB_Notebook.AddNoteItem` _output_2 _output_get_2)
                                                  (bind _output_get_3 (set `/Game/Mgnoveniye/UI/OfficeTask/WB_Notebook.NoteItemIndex` 9 _output_2))
                                                  (`/Game/Mgnoveniye/UI/OfficeTask/WB_Notebook.AddNoteItem` _output_2 _output_get_3))))))))))
                                (:`then_1`
                                  (`GameplayStatics.PlaySound2D` "/Game/Mgnoveniye/SFX/NewWAWSound/InteractWithWorld/SC_WriteNote.SC_WriteNote" 1.0 1.0 0.0 null null)
                                  (bind _foundwidgets_3 (`WidgetBlueprintLibrary.GetAllWidgetsOfClass` "/Game/Mgnoveniye/UI/OfficeTask/WB_Notebook.WB_Notebook_C"))
                                  (bind _output_3 (`|GetArrayItem` _foundwidgets_3))
                                  (`/Engine/EditorBlueprintResources/StandardMacros.IsValid` _output_3
                                    (:`Is Valid`
                                      (bind _output_get_4 (set `/Game/Mgnoveniye/UI/OfficeTask/WB_Notebook.NoteItemIndex` 6 _output_3))
                                      (`/Game/Mgnoveniye/UI/OfficeTask/WB_Notebook.AddNoteItem` _output_3 _output_get_4)
                                      (bind _output_get_5 (set `/Game/Mgnoveniye/UI/OfficeTask/WB_Notebook.NoteItemIndex` 7 _output_3))
                                      (`/Game/Mgnoveniye/UI/OfficeTask/WB_Notebook.AddNoteItem` _output_3 _output_get_5))))))))))))))))))
    (:`1`
      (bind _state_8 (`self.AddDialogue` "Марк" (select `int` (`KismetMathLibrary.RandomIntegerInRange` 0 1) :`0` "Скажи честно, мы когда-нибудь производили ножи, которые реально режут?" :`1` "Если вдруг что — я спрятался в кладовке. Психологическая разгрузка" :!type "Text") (`|MakeArray` "уйти" :!type "Text")))
      (switch `/Game/Mgnoveniye/BP/DialogueSys/Enum_DialogueState` _state_8
        (:`NewEnumerator0`
          (`self.ClearDialogueProgress`)
          (`self.CloseConversation`))))))