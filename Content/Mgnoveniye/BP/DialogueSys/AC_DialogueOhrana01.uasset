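; Dialogue component for the guard Uncle Kolya (дядя Коля), holding his Russian-language conversation with the player.
; The Dialogue override branches on DialogueTreeIndex: the first talk chains three lines, then advances the index, sets OfficeKeys on the first-person character, plays a key sound and closes.
; Later talks show one of three random greetings, then clear dialogue progress and close.
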(fn `Dialogue`
  (`parent.Dialogue`)
  (switch `int` (`self.DialogueTreeIndex`)
    (:`0`
      (bind (_state _optionindex) (`self.AddDialogue` "дядя Коля" "Доброе утро, Олег Станиславович! Опять рано на работу? Как самочувствие?" (`|MakeArray` "Доброе утро, дядя Коль. Всё отлично, спасибо. А вы как?" :!type "Text")))
      (switch `/Game/Mgnoveniye/BP/DialogueSys/Enum_DialogueState` _state
        (:`NewEnumerator0`
          (switch `int` _optionindex
            (:`0`
              _)
            (:`1`
              _))
          (bind (_state_2 _optionindex_2) (`self.AddDialogue` "дядя Коля" "Да так, сторожу порядок и вашу спину от злых бумаг" (`|MakeArray` "Спасибо, дядь Коль!" "..." :!type "Text") 1))
          (switch `/Game/Mgnoveniye/BP/DialogueSys/Enum_DialogueState` _state_2
            (:`NewEnumerator0`
              (switch `int` _optionindex_2
                (:`0`
                  _)
                (:`1`
                  _))
              (bind _state_3 (`self.AddDialogue` "дядя Коля" "Вот, ключ не забудь. Раздевалка если что открыта" (`|MakeArray` "О! Точно" "Вы заходите если что" :!type "Text")))
              (switch `/Game/Mgnoveniye/BP/DialogueSys/Enum_DialogueState` _state_3
                (:`NewEnumerator0`
                  (`self.SetDialogueTreeIndex` 1)
                  (bind _asbp_first_person_character (cast `/Game/FirstPerson/Blueprints/BP_FirstPersonCharacter` (`GameplayStatics.GetPlayerCharacter` 0)))
                  (set `/Game/FirstPerson/Blueprints/BP_FirstPersonCharacter.OfficeKeys` true _asbp_first_person_character)
                  (`GameplayStatics.PlaySound2D` "/Game/Mgnoveniye/SFX/NewWAWSound/Items/Keys_HangUp.Keys_HangUp" 1.0 1.0 0.0 null null)
                  (`self.CloseConversation`))))))))
    (:`1`
      (bind _state_4 (`self.AddDialogue` "дядя Коля" (select `int` (`KismetMathLibrary.RandomIntegerInRange` 0 2) :`0` "И снова здравствуйте, Олег Станиславович! Что-то вы к нам зачастили хахаха. Шучу-шучу" :`1` "Олег Станиславович, вы бы хоть выходной взяли…" :`2` "Как проснётесь окончательно — заходите поболтать" :!type "Text") (`|MakeArray` "Далее" :!type "Text") 1))
      (switch `/Game/Mgnoveniye/BP/DialogueSys/Enum_DialogueState` _state_4
        (:`NewEnumerator0`
          (`self.ClearDialogueProgress`)
          (`self.CloseConversation`))))))