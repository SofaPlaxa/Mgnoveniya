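; Dialogue component for the NPC Mark, holding his Russian-language office banter with the player character Oleg Stanislavovich.
; The Dialogue override branches on DialogueTreeIndex and chains AddDialogue calls into a linear conversation where reply choices do not change the path.
; Finishing it sets the index to 1, so later talks show one of two random one-liners, then clear progress and close the conversation.
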(fn `Dialogue`
  (`parent.Dialogue`)
  (switch `int` (`self.DialogueTreeIndex`)
    (:`0`
      (bind (_state _optionindex) (`self.AddDialogue` "Марк" "Ну чё, Олег Станиславович, опять в бой за великое дело пластика? \nЯ уже начинаю видеть одноразовую посуду во снах. Сегодня снилось что я ложка, как огурчик Рик, только ложка" (`|MakeArray` "А мне уже давно сны не приходят..." :!type "Text")))
      (switch `/Game/Mgnoveniye/BP/DialogueSys/Enum_DialogueState` _state
        (:`NewEnumerator0`
          (switch `int` _optionindex
            (:`0`
              _)
            (:`1`
              _))
          (bind (_state_2 _optionindex_2) (`self.AddDialogue` "Марк" "И такое бывает" (`|MakeArray` "..." :!type "Text")))
          (switch `/Game/Mgnoveniye/BP/DialogueSys/Enum_DialogueState` _state_2
            (:`NewEnumerator0`
              (switch `int` _optionindex_2
                (:`0`
                  _)
                (:`1`
                  _))
              (bind (_state_3 _optionindex_3) (`self.AddDialogue` "Марк" "Вот скажи, мы их вообще зачем носим? \n Кто-то реально думает: «О, у него на галстуке вилки — значит, он серьёзный специалист»?" (`|MakeArray` "Это часть образа. Корпоративный *стиль*. Единство. А еще они оригинальные. \nХотя на совещании я заметил, что твой галстук завязан узлом «я пытался, но устал»" :!type "Text")))
              (switch `/Game/Mgnoveniye/BP/DialogueSys/Enum_DialogueState` _state_3
                (:`NewEnumerator0`
                  (switch `int` _optionindex_3
                    (:`0`
                      _)
                    (:`1`
                      _))
                  (bind (_state_4 _optionindex_4) (`self.AddDialogue` "Марк" "Это креативный узел! Типа модный хаос. Ты посмотри на него — он, как я: странный, но старается." (`|MakeArray` " Главное, чтобы вилки не проткнули кофту. У нас же безопасность труда, всё такое." :!type "Text")))
                  (switch `/Game/Mgnoveniye/BP/DialogueSys/Enum_DialogueState` _state_4
                    (:`NewEnumerator0`
                      (switch `int` _optionindex_4
                        (:`0`
                          _)
                        (:`1`
                          _))
                      (bind (_state_5 _optionindex_5) (`self.AddDialogue` "Марк" "Легенда ты, Олег Станиславович. Камень корпоративного спокойствия.  \nКогда вырасту — хочу быть как ты. Только с нормальным галстуком" (`|MakeArray` "Все, Марк Александрович, идите работать, документы я ваши передам, спасибо" "Надо тебе иногда посерьезнее быть " :!type "Text")))
                      (switch `/Game/Mgnoveniye/BP/DialogueSys/Enum_DialogueState` _state_5
                        (:`NewEnumerator0`
                          (switch `int` _optionindex_5
                            (:`0`
                              _)
                            (:`1`
                              _))
                          (bind _state_6 (`self.AddDialogue` "Марк" "Вот и снова вошел в рабочий режим Олег Станиславович" (`|MakeArray` "..." :!type "Text")))
                          (switch `/Game/Mgnoveniye/BP/DialogueSys/Enum_DialogueState` _state_6
                            (:`NewEnumerator0`
                              (`self.SetDialogueTreeIndex` 1)
                              (`self.CloseConversation`))))))))))))))
    (:`1`
      (bind _state_7 (`self.AddDialogue` "Марк" (select `int` (`KismetMathLibrary.RandomIntegerInRange` 0 1) :`0` "Скажи честно, мы когда-нибудь производили ножи, которые реально режут?" :`1` "Если вдруг что — я спрятался в кладовке. Психологическая разгрузка" :!type "Text") (`|MakeArray` "уйти" :!type "Text")))
      (switch `/Game/Mgnoveniye/BP/DialogueSys/Enum_DialogueState` _state_7
        (:`NewEnumerator0`
          (`self.ClearDialogueProgress`)
          (`self.CloseConversation`))))))