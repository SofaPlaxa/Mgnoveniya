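; Dialogue component for the NPC "Бабка" (a grandma), holding her comedic, rude branching conversation in Russian.
; It overrides the parent Dialogue function and switches on DialogueTreeIndex, chaining AddDialogue calls by chosen option.
; In the first tree, one path advances to the second tree, while the others roll back or clear progress before closing.
; The second tree shows one of two random brush-off lines with a single exit option.
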(fn `Dialogue`
  (`parent.Dialogue`)
  (switch `int` (`self.DialogueTreeIndex`)
    (:`0`
      (bind (_state _optionindex) (`self.AddDialogue` "Бабка" "Ты че тут забыл охламон?" (`|MakeArray` "БАБКА????" "ДЕДКА????" :!type "Text")))
      (switch `/Game/Mgnoveniye/BP/DialogueSys/Enum_DialogueState` _state
        (:`NewEnumerator0`
          (switch `int` _optionindex
            (:`0`
              (bind (_state_2 _optionindex_2) (`self.AddDialogue` "Бабка" "АНУПШЕЛВОНОТСЮДА я тут тараканов ем" (`|MakeArray` "а" "чо" :!type "Text")))
              (switch `/Game/Mgnoveniye/BP/DialogueSys/Enum_DialogueState` _state_2
                (:`NewEnumerator0`
                  (switch `int` _optionindex_2
                    (:`0`
                      (bind _state_3 (`self.AddDialogue` "Бабка" "пожуй говна" (`|MakeArray` "реально бабка" "реально дедка" :!type "Text")))
                      (switch `/Game/Mgnoveniye/BP/DialogueSys/Enum_DialogueState` _state_3
                        (:`NewEnumerator0`
                          (`self.SetDialogueTreeIndex` 1)
                          (`self.CloseConversation`))))
                    (:`1`
                      (bind _state_4 (`self.AddDialogue` "Бабка" "через плечо" (`|MakeArray` ":(" :!type "Text")))
                      (switch `/Game/Mgnoveniye/BP/DialogueSys/Enum_DialogueState` _state_4
                        (:`NewEnumerator0`
                          (`self.RemoveDialogueProgress` 2)
                          (`self.CloseConversation`))))))))
            (:`1`
              (bind _state_5 (`self.AddDialogue` "Бабка" "А НИЧО ЧТО У МЕНЯ ТИТЬКИ ДО КОЛЕН" (`|MakeArray` "похоже на деда" :!type "Text")))
              (switch `/Game/Mgnoveniye/BP/DialogueSys/Enum_DialogueState` _state_5
                (:`NewEnumerator0`
                  (`self.ClearDialogueProgress`)
                  (`self.CloseConversation`))))))))
    (:`1`
      (bind _state_6 (`self.AddDialogue` "Бабка" (select `int` (`KismetMathLibrary.RandomIntegerInRange` 0 1) :`0` "че нада" :`1` "*хруст тараканов*" :!type "Text") (`|MakeArray` "уйти" :!type "Text")))
      (switch `/Game/Mgnoveniye/BP/DialogueSys/Enum_DialogueState` _state_6
        (:`NewEnumerator0`
          (`self.ClearDialogueProgress`)
          (`self.CloseConversation`))))))