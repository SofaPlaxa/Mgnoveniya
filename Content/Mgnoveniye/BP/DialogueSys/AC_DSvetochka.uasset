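; Dialogue component for the NPC Svetochka, who asks Oleg Vyacheslavovich to book a 9:30 department meeting.
; Dialogue extends the parent logic and branches on DialogueTreeIndex, with an accept or clarify choice on the first talk.
; Both choices advance the index, close the conversation and target WB_Notebook to add a task note and set GaveTask.
; Later talks replay the request until GaveTask is set, then give a random short line.
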(fn `Dialogue`
  (`parent.Dialogue`)
  (switch `int` (`self.DialogueTreeIndex`)
    (:`0`
      (bind (_state _optionindex) (`self.AddDialogue` "Светочка" "Олег Вячеславович, можете пожалуйста поставить встречу нашему отделу завтра на 9.30? " (`|MakeArray` "Без проблем" "(Уточнить)" :!type "Text") :!label _label))
      (switch `/Game/Mgnoveniye/BP/DialogueSys/Enum_DialogueState` _state
        (:`NewEnumerator0`
          (switch `int` _optionindex
            (:`0`
              (bind _state_2 (`self.AddDialogue` "Светочка" "Спасибо!" (`|MakeArray` "Далее" :!type "Text")))
              (switch `/Game/Mgnoveniye/BP/DialogueSys/Enum_DialogueState` _state_2
                (:`NewEnumerator0`
                  (`self.SetDialogueTreeIndex` 1)
                  (`self.CloseConversation`)
                  (bind _foundwidgets (`WidgetBlueprintLibrary.GetAllWidgetsOfClass` "/Game/Mgnoveniye/UI/OfficeTask/WB_Notebook.WB_Notebook_C"))
                  (bind _output (`|GetArrayItem` _foundwidgets))
                  (`/Engine/EditorBlueprintResources/StandardMacros.IsValid` _output
                    (:`Is Valid`
                      (bind _output_get (set `/Game/Mgnoveniye/UI/OfficeTask/WB_Notebook.NoteItemIndex` (`self.NoteToAddNum`) _output))
                      (`/Game/Mgnoveniye/UI/OfficeTask/WB_Notebook.AddNoteItem` _output _output_get)
                      (set `self.GaveTask` true))))))
            (:`1`
              (bind _state_3 (`self.AddDialogue` "Светочка" "Внеси нам встречу в календарь на 9.30 в среду" (`|MakeArray` "Далее" :!type "Text")))
              (switch `/Game/Mgnoveniye/BP/DialogueSys/Enum_DialogueState` _state_3
                (:`NewEnumerator0`
                  (`self.SetDialogueTreeIndex` 1)
                  (`self.CloseConversation`)
                  (bind _foundwidgets_2 (`WidgetBlueprintLibrary.GetAllWidgetsOfClass` "/Game/Mgnoveniye/UI/OfficeTask/WB_Notebook.WB_Notebook_C"))
                  (`/Engine/EditorBlueprintResources/StandardMacros.IsValid` null
                    (:`Is Valid`
                      (bind _output_2 (`|GetArrayItem` _foundwidgets_2))
                      (bind _output_get_2 (set `/Game/Mgnoveniye/UI/OfficeTask/WB_Notebook.NoteItemIndex` (`self.NoteToAddNum`) _output_2))
                      (`/Game/Mgnoveniye/UI/OfficeTask/WB_Notebook.AddNoteItem` _output_2 _output_get_2)
                      (set `self.GaveTask` true))))))))))
    (:`1`
      (if (not (`self.GaveTask`))
        (goto _label)
        (else
          (bind _state_4 (`self.AddDialogue` "Светочка" (select `int` (`KismetMathLibrary.RandomIntegerInRange` 0 1) :`0` "Я пойду дальше работать" :`1` "Еще раз спасибо!" :!type "Text") (`|MakeArray` "Далее" :!type "Text")))
          (switch `/Game/Mgnoveniye/BP/DialogueSys/Enum_DialogueState` _state_4
            (:`NewEnumerator0`
              (`self.ClearDialogueProgress`)
              (`self.CloseConversation`))))))))